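; Blueprint bridge between the app and a Node.js Neurosity script, handling account login, device selection, live device data and logout.
; UI-triggered events bind named callbacks on the NeurosityNode component, then emit credentials, the chosen nickname or a logout request.
; Script replies set variables for login status and messages, device list, state, battery, charging, and calm and focus scores.
; Empty login fields are rejected before emitting, and script console logs print to screen.
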(event OnConsoleLog(NeurosityNode)
  (params (LogMessage :type String))
  (Development|PrintString LogMessage))

(event Custom|OnCalmScore
  (params (calmScore :type String))
  ;[0.1714 0.6514 0.6445] Same as above but for the neurosityEmitter section, which receives the selected device nickname as its args in the NeurosityApp script. Just add one more Bind Event to Function and customizable event for every ipc.emit added in the script.
  (Variables|Default|SetCalmScoreMessage calmScore))

(event Custom|OnFocusScore
  (params (FocusScore :type String))
  ;[0.1714 0.6514 0.6445] Same as above but for the neurosityEmitter section, which receives the selected device nickname as its args in the NeurosityApp script. Just add one more Bind Event to Function and customizable event for every ipc.emit added in the script.
  (Variables|Default|SetFocusScoreMessage FocusScore))

(event Custom|OnChargingInfo
  (params (ChargingBoolean :type Boolean))
  ;[0.1714 0.6514 0.6445] Same as above but for the neurosityEmitter section, which receives the selected device nickname as its args in the NeurosityApp script. Just add one more Bind Event to Function and customizable event for every ipc.emit added in the script.
  (Variables|Default|SetbIsCharging ChargingBoolean))

(event Custom|OnStateInfo
  (params (StateString :type String))
  ;[0.1714 0.6514 0.6445] Same as above but for the neurosityEmitter section, which receives the selected device nickname as its args in the NeurosityApp script. Just add one more Bind Event to Function and customizable event for every ipc.emit added in the script.
  (Variables|Default|SetStateString StateString))

(event Custom|OnLoggedIn
  (params (IsLoggedIn :type Boolean))
  ;[0.1714 0.6514 0.6445] On sucessful login catch the loggedIn boolean from the script.
  (Variables|Default|SetbIsLoggedIn IsLoggedIn))

(event Custom|OnLoginClicked
  ;[1 0.4948 0.4948] SANITY CHECK : If the user submits any empty information, don't try to log in and ask first to fill the blanks. There are other foolproofs in the script in the firebaseProofer() function. Otherwise, inform the user we're attempting to log in.
  (if (or (Utilities|Array|IsEmpty (Variables|Default|GetCommitedEmail)) (Utilities|Array|IsEmpty (Variables|Default|GetCommitedPassword)))
    (Variables|Default|SetLoginErrorMessage "Please, fill in the form.")
    (Variables|Default|SetLoginButtonText "Log In")
    (else
      (Variables|Default|SetLoginErrorMessage "Please wait a few seconds.")
      (Variables|Default|SetLoginButtonText "Logging In")
      ;[1 0.5369 0.2656] Catch the login error and show it in the widget. Prompt the user to Log In again.
      (Class|NodeComponent|BindEventtoFunction (Variables|Default|GetNeurosityNode) "loginError" "OnLoginError" 0 "/")
      ;[0.1714 0.6514 0.6445] On sucessful login catch the loggedIn boolean from the script.
      (Class|NodeComponent|BindEventtoFunction (Variables|Default|GetNeurosityNode) "loggedIn" "OnLoggedIn" 0 "/")
      ;[0.1714 0.6514 0.6445] Get the deviceList string from the script.
      (Class|NodeComponent|BindEventtoFunction (Variables|Default|GetNeurosityNode) "deviceList" "OnDevicesFound" 0 "/")
      ;[0.1714 0.6514 0.6445] Make the neurosityLogger work and send the email and password string from user input. Remember, the separator is " " .
      (Class|NodeComponent|Emit (Variables|Default|GetNeurosityNode) "neurosityLogger" (Class|SIOJLibrary|ToJsonValue(String) (Utilities|String|Append (Variables|Default|GetCommitedEmail) " " (Variables|Default|GetCommitedPassword))) "/"))))

(event Custom|OnLoginError
  (params (errorMessage :type String))
  ;[1 0.5369 0.2656] Catch the login error and show it in the widget. Prompt the user to Log In again.
  (Variables|Default|SetLoginErrorMessage errorMessage)
  (Variables|Default|SetLoginButtonText "Log In"))

(event Custom|OnDevicesFound
  (params (deviceNicknames :type String))
  ;[0.1714 0.6514 0.6445] Get the deviceList string from the script.
  (Variables|Default|SetbDevicesFound true)
  (Variables|Default|SetDevicesList deviceNicknames))

(event Custom|OnNicknameSubmitted
  ;[0.1714 0.6514 0.6445] Same as above but for the neurosityEmitter section, which receives the selected device nickname as its args in the NeurosityApp script. Just add one more Bind Event to Function and customizable event for every ipc.emit added in the script.
  (Class|NodeComponent|BindEventtoFunction (Variables|Default|GetNeurosityNode) "deviceStateString" "OnStateInfo" 0 "/")
  (Class|NodeComponent|BindEventtoFunction (Variables|Default|GetNeurosityNode) "deviceBatteryInt" "OnBatteryInfo" 0 "/")
  (Class|NodeComponent|BindEventtoFunction (Variables|Default|GetNeurosityNode) "deviceChargingBool" "OnChargingInfo" 0 "/")
  (Class|NodeComponent|BindEventtoFunction (Variables|Default|GetNeurosityNode) "calmScore" "OnCalmScore" 0 "/")
  (Class|NodeComponent|BindEventtoFunction (Variables|Default|GetNeurosityNode) "focusScore" "OnFocusScore" 0 "/")
  (Class|NodeComponent|Emit (Variables|Default|GetNeurosityNode) "neurosityEmitter" (Class|SIOJLibrary|ToJsonValue(String) (Variables|Default|GetSelectedDeviceNick)) "/"))

(event Custom|OnLogoutClicked
  ;[0.1714 0.6514 0.6445] This is the logout section. No args go into this emitter. Tell the Blueprints the user is logged out and reset the login message in case the user relogs. You don't want to show them old login errors.
  (Class|NodeComponent|BindEventtoFunction (Variables|Default|GetNeurosityNode) "loggedOut" "OnLoggedOut" 0 "/")
  (Class|NodeComponent|Emit (Variables|Default|GetNeurosityNode) "neurosityLogout" 0 "/"))

(event Custom|OnLoggedOut
  (params (IsNotLoggedOut :type Boolean))
  ;[0.1714 0.6514 0.6445] This is the logout section. No args go into this emitter. Tell the Blueprints the user is logged out and reset the login message in case the user relogs. You don't want to show them old login errors.
  (Variables|Default|SetbIsLoggedIn IsNotLoggedOut)
  (Variables|Default|SetLoginErrorMessage "Use your Neurosity account login information."))

(event Custom|OnBatteryInfo
  (params (BatteryInteger :type Integer))
  ;[0.1714 0.6514 0.6445] Same as above but for the neurosityEmitter section, which receives the selected device nickname as its args in the NeurosityApp script. Just add one more Bind Event to Function and customizable event for every ipc.emit added in the script.
  (Variables|Default|SetBatteryInt BatteryInteger))

(event EventBeginPlay)

(event Collision|EventActorBeginOverlap
  (params (OtherActor :type Actor%20Object%20Reference)))

(event EventTick
  (params (DeltaSeconds :type Float%20%28single-precision%29)))

(fn ConstructionScript)